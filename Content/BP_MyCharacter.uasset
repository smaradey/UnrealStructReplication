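; Player character that moves from axis input and carries a ReplicationLog widget, apparently for displaying replication information.
; On BeginPlay it casts its Widget component's user widget to ReplicationLog and passes itself to Init, stopping if the cast fails.
; MoveForward and MoveRight add movement input along fixed world X and Y, independent of facing, with the axis value scaled by delta time and a constant.
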(event `self.ReceiveBeginPlay`
  (bind _asreplication_log (cast `/Game/ReplicationLog` (`WidgetComponent.GetUserWidgetObject` (`self.Widget`))))
  (`/Game/ReplicationLog.Init` _asreplication_log self))

(event `InputAxis|MoveForward`
  (params (AxisValue :type "Float (single-precision)"))
  (`self.AddMovementInput` (`KismetMathLibrary.MakeVector` (* AxisValue (`GameplayStatics.GetWorldDeltaSeconds`) 500.0))))

(event `InputAxis|MoveRight`
  (params (AxisValue :type "Float (single-precision)"))
  (`self.AddMovementInput` (`KismetMathLibrary.MakeVector` 0.0 (* AxisValue (`GameplayStatics.GetWorldDeltaSeconds`) 500.0))))

(fn `UserConstructionScript`)